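; Sliding door Blueprint that rises when a SideScrollerCharacter enters its Box trigger and lowers when the character leaves.
; A DoorMovement timeline plays forward or in reverse, linearly easing the Door component up to 400 units along Z.
; The offset is added to the actor location cached at BeginPlay but applied as the component's relative location.
; DoorSlideSFX activates on each trigger event and fades out when the timeline finishes.
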(event `self.ReceiveBeginPlay`
  (set `self.OriginalLocation` (`self.K2_GetActorLocation`)))

(event `self.Box.OnComponentBeginOverlap`
  (params (OverlappedComponent :type "PrimitiveComponent Object Reference") (OtherActor :type "Actor Object Reference") (OtherComp :type "PrimitiveComponent Object Reference") (OtherBodyIndex :type Integer) (bFromSweep :type Boolean) (SweepResult :type "HitResult Structure (by ref)"))
  (bind (_originallocation_x _originallocation_y _originallocation_z) (`KismetMathLibrary.BreakVector` (`self.OriginalLocation`)))
  (cast `/Game/SideScrollerBP/Blueprints/SideScrollerCharacter` OtherActor)
  (`ActorComponent.Activate` (`self.DoorSlideSFX`) true)
  (bind (_direction _newtrack_0) (`Timeline|DoorMovement` :!label _label)
    (:`Update`
      (`SceneComponent.K2_SetRelativeLocation` (`self.Door`) (`KismetMathLibrary.MakeVector` _originallocation_x _originallocation_y (+ _originallocation_z (`|EaseFunction` "Linear" _newtrack_0 0.0 400.0))) false false))
    (:`Finished`
      (`AudioComponent.FadeOut` (`self.DoorSlideSFX`) 0.5 0.0 "Linear"))))

(event `self.Box.OnComponentEndOverlap`
  (params (OverlappedComponent :type "PrimitiveComponent Object Reference") (OtherActor :type "Actor Object Reference") (OtherComp :type "PrimitiveComponent Object Reference") (OtherBodyIndex :type Integer))
  (cast `/Game/SideScrollerBP/Blueprints/SideScrollerCharacter` OtherActor)
  (`ActorComponent.Activate` (`self.DoorSlideSFX`) true)
  (goto _label :!via `Reverse`))

(fn `UserConstructionScript`)