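; Interactable button Blueprint that lets the player trigger a reactor overdrive.
; Overlapping its Box enables input and shows an InteractTooltip widget for the E key, both undone when the overlap ends.
; The Interact input action activates the overdrive sound cue, then calls ReactorOverdrive on the referenced Reactor after a fixed delay.
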(event `EnhancedInput|/Game/Input/InputMappings/Interact_IA`
  (params (ActionValue :type Boolean) (ElapsedSeconds :type "Float (double-precision)") (TriggeredSeconds :type "Float (double-precision)") (InputAction :type "InputAction Object Reference" :default "/Game/Input/InputMappings/Interact_IA.Interact_IA"))
  (:`Triggered`
    (`ActorComponent.Activate` (`self.ReactorOverdriveSFX_Cue`) false)
    (`KismetSystemLibrary.Delay` 12.0)
    (`/Game/Blueprints/Reactor.ReactorOverdrive` (`self.Reactor`))))

(event `self.Box.OnComponentBeginOverlap`
  (params (OverlappedComponent :type "PrimitiveComponent Object Reference") (OtherActor :type "Actor Object Reference") (OtherComp :type "PrimitiveComponent Object Reference") (OtherBodyIndex :type Integer) (bFromSweep :type Boolean) (SweepResult :type "HitResult Structure (by ref)"))
  (bind _returnvalue (`GameplayStatics.GetPlayerController` 0))
  (`self.EnableInput` _returnvalue)
  (bind _returnvalue_2 (`|CreateWidget` "/Game/UI/InteractTooltip.InteractTooltip_C" _returnvalue))
  (`UserWidget.AddToViewport` _returnvalue_2 0)
  (set `/Game/UI/InteractTooltip.Button` "E" _returnvalue_2)
  (set `/Game/UI/InteractTooltip.ButtonDesc` "Reactor overdrive" _returnvalue_2))

(event `self.Box.OnComponentEndOverlap`
  (params (OverlappedComponent :type "PrimitiveComponent Object Reference") (OtherActor :type "Actor Object Reference") (OtherComp :type "PrimitiveComponent Object Reference") (OtherBodyIndex :type Integer))
  (`self.DisableInput` (`GameplayStatics.GetPlayerController` 0))
  (`Widget.RemoveFromParent` (stale `self.Box.OnComponentBeginOverlap` _returnvalue_2)))

(fn `UserConstructionScript`)