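; Conveyor belt actor that carries whatever overlaps it along its forward direction.
; Each tick it offsets every overlapping actor by its forward vector scaled by Speed and delta time, without sweeping, so collisions do not block the movement.
; The construction script sizes the Box component from the InBoxExtent variable.
; The Box end-overlap event casts to FuelRod but has no further logic.
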(event `self.ReceiveTick`
  (params (DeltaSeconds :type "Float (single-precision)"))
  (for _array_element (`self.GetOverlappingActors` null)
    (`self.K2_AddActorWorldOffset` _array_element (* (`self.GetActorForwardVector`) (* DeltaSeconds (`self.Speed`))) false false)))

(event `self.Box.OnComponentEndOverlap`
  (params (OverlappedComponent :type "PrimitiveComponent Object Reference") (OtherActor :type "Actor Object Reference") (OtherComp :type "PrimitiveComponent Object Reference") (OtherBodyIndex :type Integer))
  (cast `/Game/Blueprints/FuelRod` OtherActor))

(fn `UserConstructionScript`
  (`BoxComponent.SetBoxExtent` (`self.Box`) (`self.In Box Extent`) true))